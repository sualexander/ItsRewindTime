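; BP_MenuGamemode is a menu game mode that points the player's view at the CameraActor tagged MainCamera on BeginPlay.
; Each Tick it traces under the cursor and compares the hit actor with CurrentSelection.
; The selection handling is unfinished: it assigns CurrentSelection to itself rather than the hit actor, then switches on its first tag with no cases connected.
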(event `self.ReceiveBeginPlay`
  (bind _outactors (`GameplayStatics.GetAllActorsOfClassWithTag` "/Script/Engine.CameraActor" "MainCamera"))
  (`PlayerController.SetViewTargetWithBlend` (`PlayerState.GetPlayerController` (`GameplayStatics.GetPlayerState` 0)) (`|GetArrayItem` _outactors) 0.0 "VTBlend_Linear" 0.0 false))

(event `self.ReceiveTick`
  (params (DeltaSeconds :type "Float (single-precision)"))
  (bind _currentselection (`self.CurrentSelection`))
  (bind _hitresult (`PlayerController.GetHitResultUnderCursorByChannel` (`PlayerState.GetPlayerController` (`GameplayStatics.GetPlayerState` 0)) "TraceTypeQuery3" true))
  (if (`GameplayStatics.BreakHitResult` _hitresult)
    (if (not (== _currentselection (`.HitActor` (`GameplayStatics.BreakHitResult` _hitresult))))
      (set `self.CurrentSelection` _currentselection)
      (switch `name` (`|GetArrayItem` (`Actor.Tags` _currentselection))))))

(fn `UserConstructionScript`)