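; Game mode for a turn-based rewind game, coordinating sun, music and book menu.
; Outside the overworld, it caches the sun and book and fades out all but the first forward and reversed tracks.
; Turn changes rotate and dim the sun; rewinding lerps its rotation back, adds camera motion blur and swaps music to reversed playback.
; Timelines move the book between lying, hovered and reading poses, with pause switching its page section.
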(event `self.ReceiveBeginPlay`
  (if (not (`self.isOverworld`))
    (`|ExecutionSequence`
      (:`then_0`
        (`self.InitializeStuff`))
      (:`then_1`
        (`KismetSystemLibrary.Delay` 1.0)
        (`KismetSystemLibrary.PrintString` "Fuck you motherfucker")
        (bind _asbp_rewind_game_instance (cast `/Game/Blueprints/BP_RewindGameInstance` (`GameplayStatics.GetGameInstance`))
          (:`then`
            (for (_array_element _array_index) (`/Game/Blueprints/BP_RewindGameInstance.TracksComponent` _asbp_rewind_game_instance)
              (`KismetSystemLibrary.PrintString` "Hello 1")
              (if (not (== _array_index 0))
                (`AudioComponent.AdjustVolume` _array_element 0.5 0.0 "Linear")))
            (for (_array_element_2 _array_index_2) (`/Game/Blueprints/BP_RewindGameInstance.ReversedTracksComponent` _asbp_rewind_game_instance)
              (if (not (== _array_index_2 0))
                (`AudioComponent.AdjustVolume` _array_element_2 0.5 0.0 "Linear")))
            (bind _returnvalue (`GameplayStatics.GetActorOfClass` "/Script/Engine.DirectionalLight"))
            (bind _output_get (set `self.Sun` _returnvalue))
            (set `self.BaseRotation` (`self.K2_GetActorRotation` _output_get))
            (set `self.BaseIntensity` (`LightComponentBase.Intensity` (`Light.LightComponent` _output_get))))
          (:`CastFailed`
            (`KismetSystemLibrary.PrintString` "Fucking failed casting")))))))

(event `InitializeStuff`
  (bind _bookmenuinteraction (`self.BookMenuInteraction`))
  (bind _returnvalue (`GameplayStatics.GetActorOfClass` "/Game/Blueprints/BP_RewindBook.BP_RewindBook_C"))
  (bind _output_get (set `self.Book` _returnvalue))
  (`BookMenuActor.RegisterInteractionComponent` _output_get _bookmenuinteraction)
  (`SceneComponent.K2_SetWorldTransform` _bookmenuinteraction (`KismetMathLibrary.MakeTransform` (0.0 0.0 0.0)) false true)
  (`SceneComponent.SetHiddenInGame` _bookmenuinteraction true false)
  (bind _returnvalue_2 (`GameplayStatics.GetActorOfClass` "/Game/Blueprints/BP_MenuText.BP_MenuText_C"))
  (bind _aswb_menu_text (cast `/Game/Blueprints/WB_MenuText` (`WidgetComponent.GetWidget` (`/Game/Blueprints/BP_MenuText.Widget` _returnvalue_2))))
  (bind _output_get_2 (set `self.LevelName` (`/Game/Blueprints/WB_MenuText.TextBlock_33` _aswb_menu_text)))
  (`TextBlock.SetText` _output_get_2 ""))

(event `self.OnTurnZeroUndo`
  (params (bStart :type Boolean) (NumTurns :type Integer) (Camera :type "CameraActor Object Reference"))
  (bind _currenttimelinenum (`self.CurrentTimelineNum`))
  (bind _returnvalue (+ _currenttimelinenum 1))
  (`AudioComponent.AdjustVolume` (`|GetArrayItem` (`/Game/Blueprints/BP_RewindGameInstance.TracksComponent` (stale `self.ReceiveBeginPlay` _asbp_rewind_game_instance)) _returnvalue) 1.0 0.0 "SCurve")
  (`AudioComponent.AdjustVolume` (`|GetArrayItem` (`/Game/Blueprints/BP_RewindGameInstance.ReversedTracksComponent` (stale `self.ReceiveBeginPlay` _asbp_rewind_game_instance)) _returnvalue) 1.0 0.0 "SCurve")
  (set `RewindGameInstance.currTimelineCount` _currenttimelinenum (stale `self.ReceiveBeginPlay` _asbp_rewind_game_instance)))

(event `self.OnTurnChanged`
  (params (bAdvance :type Boolean) (TurnCounter :type Integer))
  (bind _sun (`self.Sun`))
  (bind (_baserotation_roll _baserotation_pitch _baserotation_yaw) (`KismetMathLibrary.BreakRotator` (`self.BaseRotation`)))
  (bind (_returnvalue_roll _returnvalue_pitch _returnvalue_yaw) (`KismetMathLibrary.BreakRotator` (* (`self.RotationOffset`) TurnCounter)))
  (`self.K2_SetActorRotation` _sun (`KismetMathLibrary.MakeRotator` (+ _returnvalue_roll _baserotation_roll) (+ _returnvalue_pitch _baserotation_pitch) (+ _returnvalue_yaw _baserotation_yaw)) false)
  (`LightComponent.SetIntensity` (`Light.LightComponent` _sun) (- (`self.BaseIntensity`) (* TurnCounter (`self.IntensityOffset`)))))

(event `self.UpdateBook`
  (params (bOpen :type Boolean))
  (if bOpen
    (bind (_direction _newtrack_0) (`Timeline|BookPre` :!label _label)
      (:`Update`
        (`self.K2_SetActorLocation` (stale `InitializeStuff` _output_get) (`KismetMathLibrary.VLerp` (.location (`self.BookLying`)) (`self.BookHovered`) _newtrack_0) false false)))
    (else
      (goto _label :!via `Reverse`))))

(event `self.OnRewind`
  (params (bStart :type Boolean) (NumTurns :type Integer) (Camera :type "CameraActor Object Reference") (CurrTimelineNum :type Integer))
  (set `RewindGameInstance.currTimelineCount` (+ CurrTimelineNum 1) (stale `self.ReceiveBeginPlay` _asbp_rewind_game_instance))
  (if bStart
    (`|ExecutionSequence`
      (:`then_0`
        (bind _output_get (set `self.Camera` Camera))
        (setmembers `PostProcessSettings` :`StructRef` (`CameraComponent.PostProcessSettings` (`CameraActor.CameraComponent` _output_get)) :`MotionBlurAmount` 1.0 :`MotionBlurMax` 25.0 :`MotionBlurTargetFPS` 10))
      (:`then_1`
        (`TimelineComponent.SetPlayRate` (`self.Rewind`) (- 1.2 (* NumTurns 0.05)))
        (set `self.CurrentRotation` (`self.K2_GetActorRotation` (`self.Sun`)))
        (bind (_direction _alpha) (`Timeline|Rewind` :!via `PlayFromStart` :!label _label_2)
          (:`Update`
            (`self.K2_SetActorRotation` (`self.Sun`) (`KismetMathLibrary.RLerp` (`self.CurrentRotation`) (`self.BaseRotation`) _alpha) false))))
      (:`then_2`
        (`/Game/Blueprints/BP_RewindGameInstance.Start  or Stop playing for all` (stale `self.ReceiveBeginPlay` _asbp_rewind_game_instance) false (`/Game/Blueprints/BP_RewindGameInstance.TracksComponent` (stale `self.ReceiveBeginPlay` _asbp_rewind_game_instance)))
        (`/Game/Blueprints/BP_RewindGameInstance.Play at timestamp for all` (stale `self.ReceiveBeginPlay` _asbp_rewind_game_instance) true)))
    (else
      (`|ExecutionSequence`
        (:`then_0`
          (goto _label_2 :!via `Stop`))
        (:`then_1`
          (setmembers `PostProcessSettings` :`StructRef` (`CameraComponent.PostProcessSettings` (`CameraActor.CameraComponent` (`self.Camera`))) :`MotionBlurAmount` 0.5 :`MotionBlurMax` 5.0 :`MotionBlurTargetFPS` 30))
        (:`then_2`
          (`/Game/Blueprints/BP_RewindGameInstance.Start  or Stop playing for all` (stale `self.ReceiveBeginPlay` _asbp_rewind_game_instance) false (`/Game/Blueprints/BP_RewindGameInstance.ReversedTracksComponent` (stale `self.ReceiveBeginPlay` _asbp_rewind_game_instance)))
          (`/Game/Blueprints/BP_RewindGameInstance.Play at timestamp for all` (stale `self.ReceiveBeginPlay` _asbp_rewind_game_instance) false))))))

(event `self.Pause`
  (params (bStart :type Boolean))
  (bind _book (`self.Book`))
  (if bStart
    (`BookMenuActor.JumpToPageSection` _book 1)
    (bind (_direction _newtrack_0) (`Timeline|BookActual` :!label _label_3)
      (:`Update`
        (`self.K2_SetActorTransform` (`self.Book`) (`KismetMathLibrary.TLerp` (`self.BookLying`) (`self.BookReading`) _newtrack_0) false false)))
    (else
      (`BookMenuActor.JumpToPageSection` _book 0)
      (goto _label_3 :!via `Reverse`))))

(event `self.OnCollapse`)

(fn `UserConstructionScript`)