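; Game mode for a diegetic 3D main menu with Settings, Levels, Quit and Credits objects, picked by mouse.
; Tick traces under the cursor to outline the hovered actor via custom depth, aim a spotlight and label it by actor tag.
; Clicks blend to a credits camera, quit, fade exposure into the Overworld level, or lerp BP_RewindBook to reading pose for settings.
; While reading, the mouse drives a widget interaction component; Escape reverses either view.
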(event `self.ReceiveBeginPlay`
  (bind _bookmenuinteraction (`self.BookMenuInteraction`))
  (bind _returnvalue (`PlayerState.GetPlayerController` (`GameplayStatics.GetPlayerState` 0)))
  (bind _outactors (`GameplayStatics.GetAllActorsOfClassWithTag` "/Script/Engine.CameraActor" "CreditsCamera"))
  (set `self.CreditsCamera` (`|GetArrayItem` _outactors))
  (bind _outactors_2 (`GameplayStatics.GetAllActorsOfClassWithTag` "/Script/Engine.CameraActor" "MainCamera"))
  (bind _output_get (set `self.MainCamera` (`|GetArrayItem` _outactors_2)))
  (`PlayerController.SetViewTargetWithBlend` _returnvalue _output_get 0.0 "VTBlend_Linear" 0.0 false)
  (bind _returnvalue_2 (`GameplayStatics.GetActorOfClass` "/Script/Engine.SpotLight"))
  (set `self.Spotlight` _returnvalue_2)
  (set `PlayerController.bShowMouseCursor` true _returnvalue)
  (bind _returnvalue_3 (`GameplayStatics.GetActorOfClass` "/Game/Blueprints/BP_RewindBook.BP_RewindBook_C"))
  (bind _output_get_2 (set `self.Book` _returnvalue_3))
  (`BookMenuActor.RegisterInteractionComponent` _output_get_2 _bookmenuinteraction)
  (bind (_returnvalue_location _returnvalue_rotation) (`KismetMathLibrary.BreakTransform` (`self.GetTransform` _output_get_2)))
  (`SceneComponent.K2_SetWorldTransform` _bookmenuinteraction (`KismetMathLibrary.MakeTransform` (`self.K2_GetActorLocation` (`self.MainCamera`)) (* _returnvalue_rotation -1.0)) false true)
  (`SceneComponent.SetHiddenInGame` _bookmenuinteraction true false)
  (bind _returnvalue_4 (`GameplayStatics.GetActorOfClass` "/Game/Blueprints/BP_MenuText.BP_MenuText_C"))
  (bind _aswb_menu_text (cast `/Game/Blueprints/WB_MenuText` (`WidgetComponent.GetWidget` (`/Game/Blueprints/BP_MenuText.Widget` _returnvalue_4))))
  (bind _output_get_3 (set `self.MenuText` (`/Game/Blueprints/WB_MenuText.TextBlock_33` _aswb_menu_text)))
  (`TextBlock.SetText` _output_get_3 ""))

(event `self.ReceiveTick`
  (params (DeltaSeconds :type "Float (single-precision)"))
  (bind _menutext (`self.MenuText`))
  (bind _spotlight (`self.Spotlight`))
  (bind _returnvalue (`PlayerState.GetPlayerController` (`GameplayStatics.GetPlayerState` 0)))
  (bind _hitresult (`PlayerController.GetHitResultUnderCursorByChannel` _returnvalue "TraceTypeQuery3" true))
  (if (`self.bIsReading`)
    (bind (_outstart _outend) (`BookMenuStatics.CreateMouseTraceParameters` _returnvalue 5000.0)
      (:`Success`
        (`BookMenuActor.Interact` (`self.Book`) _outstart _outend false "ECC_Visibility")))
    (elif (not (== (`self.CurrentSelection`) (`.HitActor` (`GameplayStatics.BreakHitResult` _hitresult))))
      (`/Engine/EditorBlueprintResources/StandardMacros.IsValid` (`.HitActor` (`GameplayStatics.BreakHitResult` _hitresult))
        (:`Is Valid`
          (bind _output_get (set `self.CurrentSelection` (`.HitActor` (`GameplayStatics.BreakHitResult` _hitresult))))
          (`PrimitiveComponent.SetRenderCustomDepth` (`self.GetComponentByClass` _output_get "/Script/Engine.StaticMeshComponent") true)
          (`self.SetActorHiddenInGame` (`self.Spotlight`) false)
          (switch `name` (`|GetArrayItem` (`Actor.Tags` _output_get))
            (:`Settings`
              (`self.K2_SetActorRotation` _spotlight (`self.SettingsRotation`) false)
              (`TextBlock.SetText` _menutext "Settings"))
            (:`Levels`
              (`self.K2_SetActorRotation` _spotlight (`self.LevelsRotation`) false)
              (`TextBlock.SetText` _menutext "Levels"))
            (:`Quit`
              (`self.K2_SetActorRotation` _spotlight (`self.QuitRotation`) false)
              (`TextBlock.SetText` _menutext "Quit"))
            (:`Credits`
              (`self.SetActorHiddenInGame` _spotlight true)
              (`TextBlock.SetText` _menutext "Credits"))))
        (:`Is Not Valid`
          (`PrimitiveComponent.SetRenderCustomDepth` (`self.GetComponentByClass` (`self.CurrentSelection`) "/Script/Engine.StaticMeshComponent") false)
          (set `self.CurrentSelection` null)
          (`self.SetActorHiddenInGame` (`self.Spotlight`) true)
          (`TextBlock.SetText` (`self.MenuText`) ""))))))

(event `self.OnMouseClicked`
  (bind _returnvalue (`BookMenuInteractionComponent.GetWidgetInteractionComponent` (`self.BookMenuInteraction`)))
  (if (`self.bIsReading`)
    (`WidgetInteractionComponent.PressPointerKey` _returnvalue "LeftMouseButton")
    (`KismetSystemLibrary.Delay` 0.2)
    (`WidgetInteractionComponent.ReleasePointerKey` _returnvalue "LeftMouseButton")
    (else
      (bind _currentselection (`self.CurrentSelection`)
        (:`then`
          (switch `name` (`|GetArrayItem` (`Actor.Tags` _currentselection))
            (:`Settings`
              (set `self.bIsReading` true)
              (`TextBlock.SetText` (`self.MenuText`) "")
              (`self.SetActorHiddenInGame` (`self.Spotlight`) true)
              (`BookMenuActor.JumpToPageSection` (`self.Book`) 1)
              (bind (_direction _newtrack_0) (`Timeline|BookLerp` :!label _label)
                (:`Update`
                  (`self.K2_SetActorTransform` (`self.Book`) (`KismetMathLibrary.TLerp` (`self.BookLying`) (`self.BookReading`) _newtrack_0) false true))
                (:`Finished`
                  (switch `ETimelineDirection` _direction
                    (:`Backward`
                      (`KismetSystemLibrary.Delay` 0.5)
                      (set `self.CurrentSelection` null)
                      (set `self.bIsReading` false))))))
            (:`Levels`
              (`TimelineComponent.SetPlayRate` (`self.Trans`) 0.5)
              (bind (_direction_2 _newtrack_0_2) (`Timeline|Trans`)
                (:`Update`
                  (setmembers `PostProcessSettings` :`StructRef` (`CameraComponent.PostProcessSettings` (`CameraActor.CameraComponent` (`self.MainCamera`))) :`AutoExposureBias` (`KismetMathLibrary.Lerp` 10.25 40.0 _newtrack_0_2)))
                (:`Finished`
                  (`GameplayStatics.OpenLevelBySoftObjectPtr` "/Game/Overworld.Overworld"))))
            (:`Quit`
              (`KismetSystemLibrary.ExecuteConsoleCommand` "Quit" null))
            (:`Credits`
              (`PlayerController.SetViewTargetWithBlend` (`PlayerState.GetPlayerController` (`GameplayStatics.GetPlayerState` 0)) (`self.CreditsCamera`) 0.5 "VTBlend_Linear" 0.0 false))))
        (:`else`)))))

(event `self.OnEscape`
  (if (`self.bIsReading`)
    (`BookMenuActor.JumpToPageSection` (`self.Book`) 0)
    (goto _label :!via `Reverse`)
    (else
      (`PlayerController.SetViewTargetWithBlend` (`PlayerState.GetPlayerController` (`GameplayStatics.GetPlayerState` 0)) (`self.MainCamera`) 0.5 "VTBlend_Linear" 0.0 false))))

(fn `UserConstructionScript`)