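; Game instance that manages layered "Rewind Time" music as forward and reversed sets of instrument stems.
; Init creates both sets after a short delay, starts the forward one, and binds playback-percent events on one track per set to record timestamps.
; PlayAtTimestampForAll starts either set at the mirrored position (duration minus the opposite set's timestamp), muting stems indexed above CurrTimelineCount.
; A helper event toggles a given set's active state.
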(event `self.ReceiveInit`
  (`KismetSystemLibrary.Delay` 1.5)
  (`|ExecutionSequence`
    (:`then_0`
      (bind _returnvalue (`GameplayStatics.CreateSound2D` "/Game/Sounds/Music/Rewind_Time_Guitar_solo_Reversed_Track.Rewind_Time_Guitar_solo_Reversed_Track" 1.0 1.0 0.0 null true false))
      (set `self.ReversedTracksComponent` (`|MakeArray` _returnvalue (stale _returnvalue_2) (stale _returnvalue_3) (stale _returnvalue_4) (stale _returnvalue_5) (stale _returnvalue_6)) :!label _label))
    (:`then_1`
      (bind _returnvalue_2 (`GameplayStatics.CreateSound2D` "/Game/Sounds/Music/Rewind_Time_Bass_Reversed_Track.Rewind_Time_Bass_Reversed_Track" 1.0 1.0 0.0 null true false))
      (goto _label))
    (:`then_2`
      (bind _returnvalue_3 (`GameplayStatics.CreateSound2D` "/Game/Sounds/Music/Rewind_Time_Guitar_1_Reversed_Track.Rewind_Time_Guitar_1_Reversed_Track" 1.0 1.0 0.0 null true false))
      (goto _label))
    (:`then_3`
      (bind _returnvalue_4 (`GameplayStatics.CreateSound2D` "/Game/Sounds/Music/Rewind_Time_Guitar_2_Reversed_Track.Rewind_Time_Guitar_2_Reversed_Track" 1.0 1.0 0.0 null true false))
      (goto _label))
    (:`then_4`
      (bind _returnvalue_5 (`GameplayStatics.CreateSound2D` "/Game/Sounds/Music/Rewind_Time_Guitar_3_Reversed_Track.Rewind_Time_Guitar_3_Reversed_Track" 1.0 1.0 0.0 null true false))
      (goto _label))
    (:`then_5`
      (bind _returnvalue_6 (`GameplayStatics.CreateSound2D` "/Game/Sounds/Music/Rewind_Time_Guitar_4__melody__Reversed_Track.Rewind_Time_Guitar_4__melody__Reversed_Track" 1.0 1.0 0.0 null true false))
      (goto _label))
    (:`then_6`
      ;[1 1 1] Binding One Track to On Audio Playback Percent
      (add `AudioComponent.OnAudioPlaybackPercent` _returnvalue (delegate `OnAudioPlaybackPercent1`)))
    (:`then_7`
      (`KismetSystemLibrary.PrintString` "Fuck you"))
    (:`then_8`
      (`|ExecutionSequence`
        (:`then_0`
          (bind _returnvalue_7 (`GameplayStatics.CreateSound2D` "/Game/Sounds/Music/Rewind_Time_Guitar_Solo_Track.Rewind_Time_Guitar_Solo_Track" 1.0 1.0 0.0 null true false))
          (set `self.TracksComponent` (`|MakeArray` _returnvalue_7 (stale _returnvalue_8) (stale _returnvalue_9) (stale _returnvalue_10) (stale _returnvalue_11) (stale _returnvalue_12) (stale _returnvalue_13)) :!label _label_2))
        (:`then_1`
          (bind _returnvalue_8 (`GameplayStatics.CreateSound2D` "/Game/Sounds/Music/Rewind_Time_Bass_Track.Rewind_Time_Bass_Track" 1.0 1.0 0.0 null true false))
          (goto _label_2))
        (:`then_2`
          (bind _returnvalue_9 (`GameplayStatics.CreateSound2D` "/Game/Sounds/Music/Rewind_Time_Guitar_1_Track.Rewind_Time_Guitar_1_Track" 1.0 1.0 0.0 null true false))
          (goto _label_2))
        (:`then_3`
          (bind _returnvalue_10 (`GameplayStatics.CreateSound2D` "/Game/Sounds/Music/Rewind_Time_Guitar_2_Track.Rewind_Time_Guitar_2_Track" 1.0 1.0 0.0 null true false))
          (goto _label_2))
        (:`then_4`
          (bind _returnvalue_11 (`GameplayStatics.CreateSound2D` "/Game/Sounds/Music/Rewind_Time_Guitar_3_Track.Rewind_Time_Guitar_3_Track" 1.0 1.0 0.0 null true false))
          (goto _label_2))
        (:`then_5`
          (bind _returnvalue_12 (`GameplayStatics.CreateSound2D` "/Game/Sounds/Music/Rewind_Time_Guitar_4_Track_melody_.Rewind_Time_Guitar_4_Track_melody_" 1.0 1.0 0.0 null true false))
          (goto _label_2))
        (:`then_6`
          ;[1 1 1] Binding a reversed track to On Audio Playback percent
          (add `AudioComponent.OnAudioPlaybackPercent` _returnvalue_7 (delegate `OnAudioPlaybackPercent2`)))
        (:`then_7`
          (bind _returnvalue_13 (`GameplayStatics.CreateSound2D` "/Game/Sounds/Music/Rewind_Time_Pad_Track.Rewind_Time_Pad_Track" 1.0 1.0 0.0 null true false))
          (goto _label_2))
        (:`then_8`
          (for _array_element (`self.TracksComponent`)
            (`ActorComponent.SetActive` _array_element true false)
            (`AudioComponent.Play` _array_element 0.0)
            (`KismetSystemLibrary.PrintString` "Playing Init")))))))

(event `Play at timestamp for all`
  (params (Reversed :type Boolean))
  (bind _currtimelinecount (`self.currTimelineCount`))
  (`KismetSystemLibrary.PrintString` "PLay at timestamp fora ll")
  (if Reversed
    (for (_array_element _array_index) (`self.ReversedTracksComponent`)
      (`ActorComponent.SetActive` _array_element true false)
      (if (<= _array_index _currtimelinecount)
        (`KismetSystemLibrary.PrintString` "playing without mute")
        (bind _returnvalue (- (`SoundBase.Duration` (`AudioComponent.Sound` _array_element)) (`self.Timestamp`)))
        (`AudioComponent.Play` _array_element _returnvalue)
        (else
          (`AudioComponent.Play` _array_element _returnvalue)
          (`AudioComponent.AdjustVolume` _array_element 0.0 0.0 "Linear"))))
    (else
      (for (_array_element_2 _array_index_2) (`self.TracksComponent`)
        (`ActorComponent.SetActive` _array_element_2 true false)
        (if (<= _array_index_2 _currtimelinecount)
          (bind _returnvalue_2 (- (`SoundBase.Duration` (`AudioComponent.Sound` _array_element_2)) (`self.Timestamp Reversed`)))
          (`AudioComponent.Play` _array_element_2 _returnvalue_2)
          (else
            (`AudioComponent.Play` _array_element_2 _returnvalue_2)
            (`AudioComponent.AdjustVolume` _array_element_2 0.0 0.0 "Linear")))))))

(event `OnAudioPlaybackPercent1`
  (params (PlayingSoundWave :type "SoundWave Object Reference") (PlaybackPercent :type "Float (single-precision)"))
  ;[1 1 1] Binding One Track to On Audio Playback Percent
  (set `self.Timestamp Reversed` (* (`SoundBase.Duration` PlayingSoundWave) (mod PlaybackPercent 1.0))))

(event `Start  or Stop playing for all`
  (params (Start :type Boolean) (TrackComponents :type "Array of AudioComponent Object Reference"))
  (for _array_element TrackComponents
    (`ActorComponent.SetActive` _array_element Start false)))

(event `OnAudioPlaybackPercent2`
  (params (PlayingSoundWave :type "SoundWave Object Reference") (PlaybackPercent :type "Float (single-precision)"))
  ;[1 1 1] Binding a reversed track to On Audio Playback percent
  (set `self.Timestamp` (* (`SoundBase.Duration` PlayingSoundWave) (mod PlaybackPercent 1.0))))